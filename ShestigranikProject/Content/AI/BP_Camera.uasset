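; BP_Camera is an AI camera that can see the player while working and goes blind while switched off.
; StartInWork picks the initial state, and Activate and Deactivate each set the spotlight and Blind flag, then start a one-shot timer for that state's duration, apparently to alternate.
; IsSeePlayer reports a sighting only when PerceptionViewPlayer and CanSeePlayer are true and the camera is not blind.
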(event Custom|Activate
  (Rendering|Components|Light|SetIntensity (Variables|Default|GetSpotLight) 5e+05)
  (Variables|Default|SetBlind false)
  (Utilities|Time|SetTimerbyEvent (EventDispatchers|CreateEvent :!event Custom|Deactivate) (Variables|Default|GetDurationWork)))

(event Custom|Deactivate
  (Rendering|Components|Light|SetIntensity (Variables|Default|GetSpotLight) 0.0)
  (Variables|Default|SetBlind true)
  (Utilities|Time|SetTimerbyEvent (EventDispatchers|CreateEvent :!event Custom|Activate) (Variables|Default|GetDurationNotWork)))

(event EventBeginPlay
  (|CallParentFunction)
  (if (Variables|Default|GetStartInWork)
    (CallFunction|Activate)
    (else
      (CallFunction|Deactivate))))

(event Collision|EventActorBeginOverlap
  (params (OtherActor :type Actor%20Object%20Reference))
  (|CallParentFunction OtherActor) ; This node is disabled and will not be called.\nDrag off pins to build functionality.
)

(event EventTick
  (params (DeltaSeconds :type Float%20%28single-precision%29))
  (|CallParentFunction DeltaSeconds) ; This node is disabled and will not be called.\nDrag off pins to build functionality.
)

(fn ConstructionScript
  (|CallParentFunction))

(fn IsSeePlayer
  (return (Math|Boolean|ANDBoolean (Variables|Default|GetPerceptionViewPlayer) (CallFunction|CanSeePlayer) (not (Variables|Default|GetBlind)))))