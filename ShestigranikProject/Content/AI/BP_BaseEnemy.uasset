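; Base stealth enemy that patrols placed points, detects the player and fails the mission when its alarm meter fills.
; AI sight, a crouch-safe outer dark zone and a close-range check drive the meter, rising faster nearby.
; Config-based view radius and angle feed both perception and a procedural vision-cone mesh.
; Events provide external triggering, blinding, blackboard sleep, EMP/distract effects, time freezing via CustomTimeDilation and disabling.
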(event OnTargetPerceptionUpdated(AIPerception)
  (params (Actor :type Actor%20Object%20Reference) (Stimulus :type AI%20Stimulus%20Structure))
  (bind (_age _expirationage _strength _stimuluslocation _receiverlocation _tag _bsuccessfullysensed) (Utilities|Struct|BreakAIStimulus Stimulus))
  (bind _asbp_base_character (Utilities|Casting|CastToBP_BaseCharacter Actor))
  (Variables|NotEdit|SetTarget _asbp_base_character)
  (Variables|NotEdit|SetPerceptionViewPlayer _bsuccessfullysensed)
  (Variables|NotEdit|SetStimulus%20Location _stimuluslocation))

(event Custom|StartSleep
  (AI|Components|Blackboard|SetValueasBool (AI|GetBlackboard 0) (Utilities|Name|MakeLiteralName "Sleep") true))

(event Custom|EndMission
  (bind _returnvalue (Actor|GetActorOfClass "/Game/Blueprints/Core/GameFramework/BP_GameManager.BP_GameManager_C"))
  (Default|MissionFailed _returnvalue))

(event Custom|StopSleep
  (AI|Components|Blackboard|SetValueasBool (AI|GetBlackboard 0) (Utilities|Name|MakeLiteralName "Sleep") false))

(event Custom|StartEMP_FX
  (bind _returnvalue (Transformation|GetActorLocation))
  (bind _returnvalue_2 (- _returnvalue "0.000000,0.000000,88.000000"))
  (Niagara|SpawnSystematLocation "/Game/Blueprints/Niagara/NS_EMP.NS_EMP" _returnvalue_2)
  (Audio|PlaySoundatLocation "/Engine/VREditor/Sounds/UI/Dockable_Window_Drop.Dockable_Window_Drop" _returnvalue_2 "0, 0, 0" 1.0 1.0 0.0 0 0 0 0))

(event Custom|StopEMP_FX)

(event Custom|StartDistractFX
  (bind _returnvalue (Transformation|GetActorLocation))
  (Niagara|SpawnSystematLocation "/Game/Blueprints/Niagara/NS_Distract.NS_Distract" (+ _returnvalue "0.000000,0.000000,90.000000"))
  (Audio|PlaySoundatLocation "/Engine/VREditor/Sounds/UI/Floating_UI_Close-001.Floating_UI_Close-001" _returnvalue "0, 0, 0" 1.0 1.0 0.0 0 0 0 0))

(event Custom|StopDistractFX)

(event Custom|DestroyAndDisable
  (AI|Logic|StopLogic (Variables|/Script/AIModule.AIController|GetBrainComponent (AI|GetAIController self)) "")
  (Rendering|SetVisibility (Variables|Character|GetMesh) false false)
  (Collision|SetCollisionEnabled (Variables|Default|GetCapsuleComponent) "NoCollision")
  (CallFunction|StopTime))

(event EventBeginPlay
  (CallFunction|ResettoDefault)
  (CallFunction|InitPatrol)
  (CallFunction|UpdateSeePlayer false)
  (Variables|Default|SetStartPoint (Transformation|GetActorLocation))
  (Variables|Default|SetStartRot (Transformation|GetActorRotation)))

(event Collision|EventActorBeginOverlap
  (params (OtherActor :type Actor%20Object%20Reference)))

(event EventTick
  (params (DeltaSeconds :type Float%20%28single-precision%29))
  (if (Variables|NotEdit|GetAlarmInProgress)
    (CallFunction|UpdateAlarmProgress DeltaSeconds)
    (CallFunction|UpdateAlarmUI (Variables|NotEdit|GetAlarmProgress))))

(event EventTriggerEnemy
  (params (TriggerObject :type Actor%20Object%20Reference))
  (if (>= (Variables|NotEdit|GetAlarmProgress) 5e+01)
    _
    (else
      (CallFunction|SetNewAlarmValue 51.0)))
  (Variables|NotEdit|SetTargetObject TriggerObject)
  (CallFunction|GotoAlarmMode))

(event EventShowVision
  (params (Duration :type Float%20%28double-precision%29))
  (Rendering|SetVisibility (Variables|/Game/Blueprints/Game_Mechanics/BP_LineOfSight.BP_LineOfSight_C|GetProceduralMesh (Variables|NotEdit|GetAs%20BP%20Line%20Of%20Sight)) true false)
  (Utilities|FlowControl|Delay Duration)
  (CallFunction|HideVision))

(event EventHideVision
  (Rendering|SetVisibility (Variables|/Game/Blueprints/Game_Mechanics/BP_LineOfSight.BP_LineOfSight_C|GetProceduralMesh (Variables|NotEdit|GetAs%20BP%20Line%20Of%20Sight)) false false))

(event EventStartTime
  (bind _self self)
  (Variables|/Script/Engine.Actor|SetCustomTimeDilation _self 1.0)
  (Variables|/Script/Engine.Actor|SetCustomTimeDilation (AI|GetAIController _self) 1.0))

(event EventStopTime
  (bind _self self)
  (Variables|/Script/Engine.Actor|SetCustomTimeDilation _self 0.0)
  (Variables|/Script/Engine.Actor|SetCustomTimeDilation (AI|GetAIController _self) 0.0))

(fn ConstructionScript)

(fn UpdateSeePlayer
  (params (IsSeePlayer :type Boolean))
  (if IsSeePlayer
    (if (not (Variables|NotEdit|GetAlarmMode))
      (CallFunction|GotoAlarmMode))))

(fn InitPatrol
  (for _array_element (Variables|AISettings|Patrol|GetPatrolPathEditor)
    (Utilities|Array|Add (Variables|NotEdit|GetPatrolPathWorldCoordinate) (Transformation|GetActorLocation _array_element)))
  (AI|Components|Blackboard|SetValueasFloat (AI|GetBlackboard 0) (Utilities|Name|MakeLiteralName "TimeWaitOnPatrolPoint") (Variables|AISettings|Patrol|GetWaitDurationOnPatrolPoint)))

(fn GotoAlarmMode
  (Rendering|SetVisibility (Variables|Default|GetWidget) true false)
  (Rendering|SetVisibility (Variables|Default|GetBillboard) false false)
  (Variables|NotEdit|SetAlarmMode true)
  (Variables|NotEdit|SetDecrementAlarmInProgress false)
  (if (> (Variables|NotEdit|GetAlarmProgress) 0.0)
    (Variables|NotEdit|SetAlarmInProgress true)
    (else
      (bind _returnvalue (Utilities|Time|SetTimerbyFunctionName 0 "GoToAlarmInProgressMode" (Variables|AISettings|Alarm|GetDelayToProgresAlarm)))
      (Variables|NotEdit|SetAlarmInProgresDelayTimer _returnvalue))))

(fn GotoAlarminProgressMode
  (if (and (Utilities|IsValid (Variables|NotEdit|GetTarget)) (Variables|NotEdit|GetAlarmMode))
    (Variables|NotEdit|SetAlarmInProgress true)))

(fn GotoNormalMode
  (Variables|NotEdit|SetAlarmMode false)
  (Variables|NotEdit|SetAlarmInProgress false)
  (Utilities|Time|ClearandInvalidateTimerbyHandle (Variables|NotEdit|GetAlarmInProgresDelayTimer))
  (Rendering|SetVisibility (Variables|Default|GetBillboard) false false)
  (CallFunction|ResetSecondTarget))

(fn UpdateAlarmProgress
  (params (DeltaSeconds :type Float%20%28double-precision%29))
  (bind _returnvalue (Utilities|GetNewIncrementAlarmValue DeltaSeconds))
  (if (CallFunction|IsSeePlayer)
    (CallFunction|SetNewAlarmValue _returnvalue)
    (if (>= _returnvalue 1e+02)
      (CallFunction|EndMission))
    (elif (> (Variables|NotEdit|GetAlarmProgress) 0.0)
      (if (Variables|NotEdit|GetDecrementAlarmInProgress)
        (CallFunction|SetNewAlarmValue (Utilities|GetNewDecrementAlarmValue DeltaSeconds)))
      (else
        (CallFunction|GotoNormalMode)
        (Rendering|SetVisibility (Variables|Default|GetWidget) false false)))))

(fn GetSpeedIncrementAlarm
  (Utilities|IsValid (Variables|NotEdit|GetTarget)
    (:Is%20Valid
      (return (* (Variables|AISettings|Alarm|GetMinSpeedAlarm) (/ (Variables|AISettings|ViewZone|GetMaxViewRadius) (Utilities|GetDistancetoTarget)))))
    (:Is%20Not%20Valid
      (return 0.0))))

(fn GetSpeedDecrementAlarm
  (return 1e+01))

(fn InitPerception
  (Class|AIHelperLib|SetAISightPerception (Variables|Default|GetAIPerception) (Variables|AISettings|ViewZone|GetMaxViewRadius) (/ (Variables|AISettings|ViewZone|GetAngleView) 2.0)))

(fn UpdateAlarmUI
  (params (AlarmProgress :type Float%20%28double-precision%29))
  (bind _aswbp_aistatus (Utilities|Casting|CastToWBP_AIStatus (UserInterface|GetWidget (Variables|Default|GetWidget))))
  (Default|UpdateAlarm _aswbp_aistatus AlarmProgress))

(fn CanSeePlayer
  (Utilities|IsValid (Variables|NotEdit|GetTarget)
    (:Is%20Valid
      (return (not (and (Utilities|IsDarkZone (Utilities|GetDistancetoTarget)) (Class|BaseCharacter|IsCrouch (Variables|NotEdit|GetTarget))))))
    (:Is%20Not%20Valid
      (return false))))

(fn ShowTargetPoint
  (bind _outactors (Actor|GetAllActorsOfClass "/Game/AI/BP_PatrolPoint.BP_PatrolPoint_C"))
  (for _array_element _outactors
    (Default|SetVisibility _array_element false))
  (for _array_element_2 (Variables|AISettings|Patrol|GetPatrolPathEditor)
    (Default|SetVisibility _array_element_2 true)))

(fn IsSeePlayer
  (return (or (Math|Boolean|ANDBoolean (Variables|NotEdit|GetPerceptionViewPlayer) (CallFunction|CanSeePlayer) (not (Variables|Default|GetBlind))) (CallFunction|CheckNearlySeePlayer))))

(fn InitLineOfSight
  (bind _asbp_line_of_sight (Utilities|Casting|CastToBP_LineOfSight (Variables|/Script/Engine.ChildActorComponent|GetChildActor (Variables|Default|GetLineOfSight))))
  (bind _output_get (Variables|NotEdit|SetAs%20BP%20Line%20Of%20Sight _asbp_line_of_sight))
  (Default|Initizialize (Variables|NotEdit|GetAs%20BP%20Line%20Of%20Sight) (/ (Variables|AISettings|ViewZone|GetAngleView) 2.0) (Variables|AISettings|ViewZone|GetMaxViewRadius) (* (Variables|AISettings|ViewZone|GetMaxViewRadius) (- 1.0 (Variables|AISettings|ViewZone|GetDarkZonePercent))))
  (Rendering|SetVisibility (Variables|/Game/Blueprints/Game_Mechanics/BP_LineOfSight.BP_LineOfSight_C|GetProceduralMesh _output_get) false false))

(fn SetNewAlarmValue
  (params (AlarmProgress :type Float%20%28double-precision%29))
  (bind _output_get (Variables|NotEdit|SetAlarmProgress AlarmProgress))
  (CallFunction|UpdateAlarmUI _output_get))

(fn ResetSecondTarget
  (Variables|NotEdit|SetTargetObject 0))

(fn CheckNearlySeePlayer
  (bind _target (Variables|NotEdit|GetTarget))
  (Utilities|IsValid _target
    (:Is%20Valid
      (return (< (Math|Vector|Distance2D(Vector) (Transformation|GetActorLocation _target) (Transformation|GetActorLocation)) 1e+02)))
    (:Is%20Not%20Valid
      (return false))))

(fn SetBlinded
  (params (duration :type Float%20%28double-precision%29))
  (Variables|Default|SetBlind true)
  (Utilities|Time|SetTimerbyEvent (EventDispatchers|CreateEvent :!event ResetBlinded) duration))

(fn ResetBlinded
  (Variables|Default|SetBlind false))

(fn UpdateViewRadius
  (params (Radius :type Float%20%28double-precision%29))
  (Variables|AISettings|ViewZone|SetMaxViewRadius Radius)
  (bind _asbp_line_of_sight (Utilities|Casting|CastToBP_LineOfSight (Variables|/Script/Engine.ChildActorComponent|GetChildActor (Variables|Default|GetLineOfSight))))
  (Default|SetNewRadius _asbp_line_of_sight (Variables|AISettings|ViewZone|GetMaxViewRadius) (* (Variables|AISettings|ViewZone|GetMaxViewRadius) (- 1.0 (Variables|AISettings|ViewZone|GetDarkZonePercent)))))

(fn ResettoDefault
  (bind _defaultenemyconfig (Variables|AISettings|GetDefaultEnemyConfig))
  (bind (_maxviewradius _angleview) (Utilities|Struct|BreakST_Enemy _defaultenemyconfig))
  (Variables|AISettings|ViewZone|SetMaxViewRadius _maxviewradius)
  (Variables|AISettings|ViewZone|SetAngleView _angleview)
  (CallFunction|InitLineOfSight)
  (CallFunction|InitPerception))