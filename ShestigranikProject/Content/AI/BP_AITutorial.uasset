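; BP_AITutorial is an AI Blueprint, apparently for a tutorial, that resets the situation when its mission ends.
; Its EndMission event teleports a valid Target to the RespawnPoint's location and rotation, then sets the alarm value to zero through SetNewAlarmValue.
; The default BeginPlay, overlap and Tick events are disabled stubs, so EndMission is the only active logic in this graph.
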(event EventBeginPlay
  (|CallParentFunction) ; This node is disabled and will not be called.\nDrag off pins to build functionality.
)

(event Collision|EventActorBeginOverlap
  (params (OtherActor :type Actor%20Object%20Reference))
  (|CallParentFunction OtherActor) ; This node is disabled and will not be called.\nDrag off pins to build functionality.
)

(event EventTick
  (params (DeltaSeconds :type Float%20%28single-precision%29))
  (|CallParentFunction DeltaSeconds) ; This node is disabled and will not be called.\nDrag off pins to build functionality.
)

(event EventEndMission
  (bind _respawnpoint (Variables|Default|GetRespawnPoint))
  (bind _target (Variables|Default|GetTarget))
  (bind _returnvalue (Transformation|GetActorTransform _respawnpoint))
  (Utilities|IsValid _target
    (:Is%20Valid
      (Transformation|SetActorLocationAndRotation _target (.location _returnvalue) (.rotation _returnvalue))
      (CallFunction|SetNewAlarmValue 0.0))))

(fn ConstructionScript
  (|CallParentFunction))