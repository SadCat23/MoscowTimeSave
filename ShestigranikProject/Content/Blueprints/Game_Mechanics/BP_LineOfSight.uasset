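; Line-of-sight actor that draws a field-of-view cone as a procedural mesh, showing visible and cover zones.
; Once initialized, each Tick clears the mesh and fans line traces across the view angle.
; Optional bisection tracing sharpens edges where the hit actor changes.
; Hits become visible-zone triangles; behind obstacles not tagged "High", a raised second trace bounds cover-zone sections, each zone using its own dynamic material.
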(event EventBeginPlay)

(event Collision|EventActorBeginOverlap
  (params (OtherActor :type Actor%20Object%20Reference)))

(event EventTick
  (params (DeltaSeconds :type Float%20%28single-precision%29))
  (if (Variables|Default|Getinit)
    (CallFunction|Update)
    (CallFunction|LineTracing)))

(fn ConstructionScript
  (if (Variables|Debug|GetRebuild)
    (CallFunction|Initizialize (Variables|FieldOfVision|GetHalfAngle) (Variables|FieldOfVision|GetExternalRadius) (Variables|FieldOfVision|GetInternalRadiusOvVisibility))
    (CallFunction|Start)
    (CallFunction|LineTracing)))

(fn CreateProceduralMesh
  (Rendering|SetCastShadow (Variables|Default|GetProceduralMesh) false)
  ;[1 1 1] MaterialSetup
  (bind _returnvalue (Rendering|Material|CreateDynamicMaterialInstance "/Game/Materials/LineOfSight/MI_VisibleZone.MI_VisibleZone" "None" "None" :!class /Script/Engine.KismetMaterialLibrary))
  (bind _output_get (LocalVariables|SetVisibleZoneMatInst _returnvalue))
  (Rendering|Material|SetVectorParameterValue _output_get "Center" (Math|Conversions|ToLinearColor(Vector) (Transformation|GetActorLocation)) :!class /Script/Engine.MaterialInstanceDynamic)
  (Rendering|Material|SetScalarParameterValue _output_get "ViewDistance" (Variables|FieldOfVision|GetInternalRadiusOvVisibility) :!class /Script/Engine.MaterialInstanceDynamic)
  (bind _returnvalue_2 (Rendering|Material|CreateDynamicMaterialInstance "/Game/Materials/LineOfSight/MI_CoverZone.MI_CoverZone" "None" "None" :!class /Script/Engine.KismetMaterialLibrary))
  (bind _output_get_2 (LocalVariables|SetCoverZoneMatInst _returnvalue_2))
  (Rendering|Material|SetVectorParameterValue _output_get_2 "Center" (Math|Conversions|ToLinearColor(Vector) (Transformation|GetActorLocation)) :!class /Script/Engine.MaterialInstanceDynamic)
  (Rendering|Material|SetScalarParameterValue _output_get_2 "ViewDistance" (Variables|FieldOfVision|GetInternalRadiusOvVisibility) :!class /Script/Engine.MaterialInstanceDynamic)
  ;[0.4677 1 0.2155] VisibleZones
  (if (Variables|FieldOfVision|GetUseExternalPrecise)
    (CallFunction|PreciseExternalBorders))
  (for _index (range 0 (- (Utilities|Array|LastIndex (Variables|Auxiliary|GetHitResults)) 1))
    (LocalVariables|SetI _index)
    (Utilities|FlowControl|Sequence
      (:then_0
        (if (.bBlockingHit (Collision|BreakHitResult (Utilities|Array|Get(acopy) (Variables|Auxiliary|GetHitResults) (LocalVariables|GetI))))
          (LocalVariables|SetLLeftPoint (.Location (Collision|BreakHitResult (Utilities|Array|Get(acopy) (Variables|Auxiliary|GetHitResults) (LocalVariables|GetI)))))
          (LocalVariables|SetNeedLeftAdditive (not (Actor|ActorHasTag (.HitActor (Collision|BreakHitResult (Utilities|Array|Get(acopy) (Variables|Auxiliary|GetHitResults) (LocalVariables|GetI)))) "High")))
          (if (.bBlockingHit (CallFunction|CheckActorHigh (Utilities|Array|Get(acopy) (Variables|Auxiliary|GetHitResults) (LocalVariables|GetI))))
            (LocalVariables|SetLLeftFarPoint (.Location (CallFunction|CheckActorHigh (Utilities|Array|Get(acopy) (Variables|Auxiliary|GetHitResults) (LocalVariables|GetI)))))
            (else
              (LocalVariables|SetLLeftFarPoint (.TraceEnd (Collision|BreakHitResult (Utilities|Array|Get(acopy) (Variables|Auxiliary|GetHitResults) (LocalVariables|GetI)))))))
          (else
            (LocalVariables|SetLLeftPoint (.TraceEnd (Collision|BreakHitResult (Utilities|Array|Get(acopy) (Variables|Auxiliary|GetHitResults) (LocalVariables|GetI)))))
            (LocalVariables|SetNeedLeftAdditive false))))
      (:then_1
        (if (.bBlockingHit (Collision|BreakHitResult (Utilities|Array|Get(acopy) (Variables|Auxiliary|GetHitResults) (+ (LocalVariables|GetI) 1))))
          (LocalVariables|SetLRightPoint (.Location (Collision|BreakHitResult (Utilities|Array|Get(acopy) (Variables|Auxiliary|GetHitResults) (+ (LocalVariables|GetI) 1)))))
          (LocalVariables|SetNeedRightAdditive (not (Actor|ActorHasTag (.HitActor (Collision|BreakHitResult (Utilities|Array|Get(acopy) (Variables|Auxiliary|GetHitResults) (+ (LocalVariables|GetI) 1)))) "High")))
          (if (.bBlockingHit (CallFunction|CheckActorHigh (Utilities|Array|Get(acopy) (Variables|Auxiliary|GetHitResults) (+ (LocalVariables|GetI) 1))))
            (LocalVariables|SetLRightFarPoint (.Location (CallFunction|CheckActorHigh (Utilities|Array|Get(acopy) (Variables|Auxiliary|GetHitResults) (+ (LocalVariables|GetI) 1)))))
            (else
              (LocalVariables|SetLRightFarPoint (.TraceEnd (Collision|BreakHitResult (Utilities|Array|Get(acopy) (Variables|Auxiliary|GetHitResults) (+ (LocalVariables|GetI) 1)))))))
          (else
            (LocalVariables|SetLRightPoint (.TraceEnd (Collision|BreakHitResult (Utilities|Array|Get(acopy) (Variables|Auxiliary|GetHitResults) (+ (LocalVariables|GetI) 1)))))
            (LocalVariables|SetNeedRightAdditive false))))
      (:then_2
        (Class|ProceduralMeshComponent|CreateMeshSectionLinearColor (Variables|Default|GetProceduralMesh) (LocalVariables|GetI) (Utilities|Array|MakeArray "0, 0, 0" (- (LocalVariables|GetLLeftPoint) (Variables|Auxiliary|GetStartPoint)) (- (LocalVariables|GetLRightPoint) (Variables|Auxiliary|GetStartPoint))) (Utilities|Array|MakeArray 0 2 1) 0 (Utilities|Array|MakeArray "(X=0.500000,Y=0.500000)" (Math|Vector2D|MakeVector2D (.x (+ (/ (/ (- (LocalVariables|GetLLeftPoint) (Variables|Auxiliary|GetStartPoint)) (Variables|FieldOfVision|GetExternalRadius)) 2.0) 0.5)) (.y (+ (/ (/ (- (LocalVariables|GetLLeftPoint) (Variables|Auxiliary|GetStartPoint)) (Variables|FieldOfVision|GetExternalRadius)) 2.0) 0.5))) (Math|Vector2D|MakeVector2D (.x (+ (/ (/ (- (LocalVariables|GetLRightPoint) (Variables|Auxiliary|GetStartPoint)) (Variables|FieldOfVision|GetExternalRadius)) 2.0) 0.5)) (.y (+ (/ (/ (- (LocalVariables|GetLRightPoint) (Variables|Auxiliary|GetStartPoint)) (Variables|FieldOfVision|GetExternalRadius)) 2.0) 0.5)))) 0 0 0 0 0 false false)
        (Rendering|Material|SetMaterial (Variables|Default|GetProceduralMesh) (LocalVariables|GetI) (LocalVariables|GetVisibleZoneMatInst))
        ;[1 0.3829 0] InvisibleZones
        (Utilities|FlowControl|Sequence
          (:then_0
            (if (and (LocalVariables|GetNeedLeftAdditive) (not (LocalVariables|GetNeedRightAdditive)))
              (Class|ProceduralMeshComponent|CreateMeshSectionLinearColor (Variables|Default|GetProceduralMesh) (+ (- (Utilities|Array|LastIndex (Variables|Auxiliary|GetHitResults)) 1) (LocalVariables|GetI)) (Utilities|Array|MakeArray (- (LocalVariables|GetLLeftPoint) (Variables|Auxiliary|GetStartPoint)) (- (LocalVariables|GetLLeftFarPoint) (Variables|Auxiliary|GetStartPoint)) (- (LocalVariables|GetLRightPoint) (Variables|Auxiliary|GetStartPoint))) (Utilities|Array|MakeArray 0 2 1) 0 (Utilities|Array|MakeArray (Math|Vector2D|MakeVector2D (.x (+ (/ (/ (- (LocalVariables|GetLLeftPoint) (Variables|Auxiliary|GetStartPoint)) (Variables|FieldOfVision|GetExternalRadius)) 2.0) 0.5)) (.y (+ (/ (/ (- (LocalVariables|GetLLeftPoint) (Variables|Auxiliary|GetStartPoint)) (Variables|FieldOfVision|GetExternalRadius)) 2.0) 0.5))) (Math|Vector2D|MakeVector2D (.x (+ (/ (/ (- (LocalVariables|GetLLeftFarPoint) (Variables|Auxiliary|GetStartPoint)) (Variables|FieldOfVision|GetExternalRadius)) 2.0) 0.5)) (.y (+ (/ (/ (- (LocalVariables|GetLLeftFarPoint) (Variables|Auxiliary|GetStartPoint)) (Variables|FieldOfVision|GetExternalRadius)) 2.0) 0.5))) (Math|Vector2D|MakeVector2D (.x (+ (/ (/ (- (LocalVariables|GetLRightPoint) (Variables|Auxiliary|GetStartPoint)) (Variables|FieldOfVision|GetExternalRadius)) 2.0) 0.5)) (.y (+ (/ (/ (- (LocalVariables|GetLRightPoint) (Variables|Auxiliary|GetStartPoint)) (Variables|FieldOfVision|GetExternalRadius)) 2.0) 0.5)))) 0 0 0 0 0 false false)
              (Rendering|Material|SetMaterial (Variables|Default|GetProceduralMesh) (+ (- (Utilities|Array|LastIndex (Variables|Auxiliary|GetHitResults)) 1) (LocalVariables|GetI)) (LocalVariables|GetCoverZoneMatInst))))
          (:then_1
            (if (and (LocalVariables|GetNeedRightAdditive) (not (LocalVariables|GetNeedLeftAdditive)))
              (Class|ProceduralMeshComponent|CreateMeshSectionLinearColor (Variables|Default|GetProceduralMesh) (+ (- (Utilities|Array|LastIndex (Variables|Auxiliary|GetHitResults)) 1) (LocalVariables|GetI)) (Utilities|Array|MakeArray (- (LocalVariables|GetLRightPoint) (Variables|Auxiliary|GetStartPoint)) (- (LocalVariables|GetLLeftPoint) (Variables|Auxiliary|GetStartPoint)) (- (LocalVariables|GetLRightFarPoint) (Variables|Auxiliary|GetStartPoint))) (Utilities|Array|MakeArray 0 2 1) 0 (Utilities|Array|MakeArray (Math|Vector2D|MakeVector2D (.x (+ (/ (/ (- (LocalVariables|GetLRightPoint) (Variables|Auxiliary|GetStartPoint)) (Variables|FieldOfVision|GetExternalRadius)) 2.0) 0.5)) (.y (+ (/ (/ (- (LocalVariables|GetLRightPoint) (Variables|Auxiliary|GetStartPoint)) (Variables|FieldOfVision|GetExternalRadius)) 2.0) 0.5))) (Math|Vector2D|MakeVector2D (.x (+ (/ (/ (- (LocalVariables|GetLLeftPoint) (Variables|Auxiliary|GetStartPoint)) (Variables|FieldOfVision|GetExternalRadius)) 2.0) 0.5)) (.y (+ (/ (/ (- (LocalVariables|GetLLeftPoint) (Variables|Auxiliary|GetStartPoint)) (Variables|FieldOfVision|GetExternalRadius)) 2.0) 0.5))) (Math|Vector2D|MakeVector2D (.x (+ (/ (/ (- (LocalVariables|GetLRightFarPoint) (Variables|Auxiliary|GetStartPoint)) (Variables|FieldOfVision|GetExternalRadius)) 2.0) 0.5)) (.y (+ (/ (/ (- (LocalVariables|GetLRightFarPoint) (Variables|Auxiliary|GetStartPoint)) (Variables|FieldOfVision|GetExternalRadius)) 2.0) 0.5)))) 0 0 0 0 0 false false)
              (Rendering|Material|SetMaterial (Variables|Default|GetProceduralMesh) (+ (- (Utilities|Array|LastIndex (Variables|Auxiliary|GetHitResults)) 1) (LocalVariables|GetI)) (LocalVariables|GetCoverZoneMatInst))))
          (:then_2
            (if (and (LocalVariables|GetNeedRightAdditive) (LocalVariables|GetNeedLeftAdditive))
              (Class|ProceduralMeshComponent|CreateMeshSectionLinearColor (Variables|Default|GetProceduralMesh) (+ (- (Utilities|Array|LastIndex (Variables|Auxiliary|GetHitResults)) 1) (LocalVariables|GetI)) (Utilities|Array|MakeArray (- (LocalVariables|GetLRightPoint) (Variables|Auxiliary|GetStartPoint)) (- (LocalVariables|GetLRightFarPoint) (Variables|Auxiliary|GetStartPoint)) (- (LocalVariables|GetLLeftFarPoint) (Variables|Auxiliary|GetStartPoint)) (- (LocalVariables|GetLLeftPoint) (Variables|Auxiliary|GetStartPoint))) (Utilities|Array|MakeArray 0 2 3 0 1 2) 0 (Utilities|Array|MakeArray (Math|Vector2D|MakeVector2D (.x (+ (/ (/ (- (LocalVariables|GetLRightPoint) (Variables|Auxiliary|GetStartPoint)) (Variables|FieldOfVision|GetExternalRadius)) 2.0) 0.5)) (.y (+ (/ (/ (- (LocalVariables|GetLRightPoint) (Variables|Auxiliary|GetStartPoint)) (Variables|FieldOfVision|GetExternalRadius)) 2.0) 0.5))) (Math|Vector2D|MakeVector2D (.x (+ (/ (/ (- (LocalVariables|GetLRightFarPoint) (Variables|Auxiliary|GetStartPoint)) (Variables|FieldOfVision|GetExternalRadius)) 2.0) 0.5)) (.y (+ (/ (/ (- (LocalVariables|GetLRightFarPoint) (Variables|Auxiliary|GetStartPoint)) (Variables|FieldOfVision|GetExternalRadius)) 2.0) 0.5))) (Math|Vector2D|MakeVector2D (.x (+ (/ (/ (- (LocalVariables|GetLLeftFarPoint) (Variables|Auxiliary|GetStartPoint)) (Variables|FieldOfVision|GetExternalRadius)) 2.0) 0.5)) (.y (+ (/ (/ (- (LocalVariables|GetLLeftFarPoint) (Variables|Auxiliary|GetStartPoint)) (Variables|FieldOfVision|GetExternalRadius)) 2.0) 0.5))) (Math|Vector2D|MakeVector2D (.x (+ (/ (/ (- (LocalVariables|GetLLeftPoint) (Variables|Auxiliary|GetStartPoint)) (Variables|FieldOfVision|GetExternalRadius)) 2.0) 0.5)) (.y (+ (/ (/ (- (LocalVariables|GetLLeftPoint) (Variables|Auxiliary|GetStartPoint)) (Variables|FieldOfVision|GetExternalRadius)) 2.0) 0.5)))) 0 0 0 0 0 false false)
              (Rendering|Material|SetMaterial (Variables|Default|GetProceduralMesh) (+ (- (Utilities|Array|LastIndex (Variables|Auxiliary|GetHitResults)) 1) (LocalVariables|GetI)) (LocalVariables|GetCoverZoneMatInst))))))))
  (Transformation|SetRelativeRotation (Variables|Default|GetProceduralMesh) (* (Math|Rotator|MakeRotfromX (Transformation|GetActorForwardVector)) -1.0) false false))

(fn PreciseExternalBorders
  (for _index (range 0 (- (Utilities|Array|LastIndex (Variables|Auxiliary|GetHitResults)) 0))
    (LocalVariables|SetI _index)
    (Utilities|Array|Add (LocalVariables|GetLHitResults) (Utilities|Array|Get(acopy) (Variables|Auxiliary|GetHitResults) (LocalVariables|GetI)))
    (if (!= (.HitActor (Collision|BreakHitResult (Utilities|Array|Get(acopy) (Variables|Auxiliary|GetHitResults) (LocalVariables|GetI)))) (.HitActor (Collision|BreakHitResult (Utilities|Array|Get(acopy) (Variables|Auxiliary|GetHitResults) (+ (LocalVariables|GetI) 1)))))
      (Utilities|FlowControl|Sequence
        (:then_0
          (if (.bBlockingHit (Collision|BreakHitResult (Utilities|Array|Get(acopy) (Variables|Auxiliary|GetHitResults) (LocalVariables|GetI))))
            (LocalVariables|SetLLeftPoint (.Location (Collision|BreakHitResult (Utilities|Array|Get(acopy) (Variables|Auxiliary|GetHitResults) (LocalVariables|GetI)))))
            (else
              (LocalVariables|SetLLeftPoint (.TraceEnd (Collision|BreakHitResult (Utilities|Array|Get(acopy) (Variables|Auxiliary|GetHitResults) (LocalVariables|GetI))))))))
        (:then_1
          (if (.bBlockingHit (Collision|BreakHitResult (Utilities|Array|Get(acopy) (Variables|Auxiliary|GetHitResults) (+ (LocalVariables|GetI) 1))))
            (LocalVariables|SetLRightPoint (.Location (Collision|BreakHitResult (Utilities|Array|Get(acopy) (Variables|Auxiliary|GetHitResults) (+ (LocalVariables|GetI) 1)))))
            (else
              (LocalVariables|SetLRightPoint (.TraceEnd (Collision|BreakHitResult (Utilities|Array|Get(acopy) (Variables|Auxiliary|GetHitResults) (+ (LocalVariables|GetI) 1))))))))
        (:then_2
          (bind _outhits (CallFunction|BisectionMethod (LocalVariables|GetLLeftPoint) (LocalVariables|GetLRightPoint) (Variables|Auxiliary|GetStartPoint) (.HitActor (Collision|BreakHitResult (Utilities|Array|Get(acopy) (Variables|Auxiliary|GetHitResults) (LocalVariables|GetI)))) (.HitActor (Collision|BreakHitResult (Utilities|Array|Get(acopy) (Variables|Auxiliary|GetHitResults) (+ (LocalVariables|GetI) 1))))))
          (for _array_element _outhits
            (Utilities|Array|Add (LocalVariables|GetLHitResults) _array_element))))))
  (Utilities|Array|Add (LocalVariables|GetLHitResults) (Utilities|Array|Get(acopy) (Variables|Auxiliary|GetHitResults) (Utilities|Array|LastIndex (Variables|Auxiliary|GetHitResults))))
  (Variables|Auxiliary|SetHitResults (LocalVariables|GetLHitResults)))

(fn LineTracing
  (bind _startpoint (Variables|Auxiliary|GetStartPoint))
  (for _index (range 0 (Variables|Auxiliary|GetNumberOfSections))
    (LocalVariables|SetLCurrentAngle (- (* _index (Variables|Default|GetDAngle)) (Variables|FieldOfVision|GetHalfAngle)))
    (bind _outhit (Collision|LineTraceByChannel _startpoint (+ _startpoint (* (Math|Vector|RotateVectorAroundAxis (Transformation|GetActorForwardVector) (LocalVariables|GetLCurrentAngle) "0.000000,0.000000,1.000000") (Variables|FieldOfVision|GetExternalRadius))) "TraceTypeQuery1" false 0 (Variables|Debug|GetDrawDebugType) true "(R=1.000000,G=0.000000,B=0.000000,A=1.000000)" "(R=0.000000,G=1.000000,B=0.000000,A=1.000000)" (Variables|Debug|GetDraw%20Time)))
    (Utilities|Array|Add (Variables|Auxiliary|GetHitResults) _outhit))
  (CallFunction|CreateProceduralMesh))

(fn Start
  (Utilities|FlowControl|Sequence
    (:then_0
      (bind _output_get (Variables|Auxiliary|SetNumberOfSections (Math|Float|Ceil (/ (* (Variables|FieldOfVision|GetHalfAngle) 2.0) (Variables|FieldOfVision|GetDeltaAngle)))))
      (Variables|Default|SetDAngle (/ (* (Variables|FieldOfVision|GetHalfAngle) 2.0) _output_get)))
    (:then_1
      (Variables|Auxiliary|SetStartPoint (+ (Math|Vector|MakeVector 0.0 0.0 (- (Variables|FieldOfVision|GetHeightOfCheck) 1e+02)) (Transformation|GetActorLocation))))
    (:then_2
      (Transformation|AddLocalOffset (Variables|Default|GetProceduralMesh) (Math|Vector|MakeVector 0.0 0.0 (- (Variables|FieldOfVision|GetHeightOfCheck) 1e+02)) false false))))

(fn BisectionMethod
  (params (LeftPoint :type Vector) (RightPoint :type Vector) (StartPoint :type Vector) (LeftActor :type Actor%20Object%20Reference) (RightActor :type Actor%20Object%20Reference))
  (bind _returnvalue (- RightPoint StartPoint))
  (bind _lotheractors (LocalVariables|GetLOtherActors))
  ;[1 1 1] Init
  (LocalVariables|SetLLeftDirection (- LeftPoint StartPoint))
  (LocalVariables|SetLRightDirection _returnvalue)
  (LocalVariables|SetLStartPoint StartPoint)
  (LocalVariables|SetLLeftActor LeftActor)
  (LocalVariables|SetLRightVector RightActor)
  (LocalVariables|SetLCurrentAngle (Variables|FieldOfVision|GetPreciseAngle) :!label _label)
  (LocalVariables|SetCount 0)
  (while (and (<= (- (Variables|FieldOfVision|GetPreciseAngle) (LocalVariables|GetLCurrentAngle)) 0.0) (<= (LocalVariables|GetCount) (Variables|Debug|GetPreciseCount)))
    (Math|Integer|IncrementInt (LocalVariables|GetCount)
      (:%20%20
        (LocalVariables|SetLCurrentAngle (Math|Float|Absolute(Float) (* (- (.Yaw (Math|Rotator|BreakRotator (Math|Rotator|MakeRotfromX (LocalVariables|GetLLeftDirection)))) (.Yaw (Math|Rotator|BreakRotator (Math|Rotator|MakeRotfromX (LocalVariables|GetLRightDirection))))) 0.5)))
        (LocalVariables|SetLMidDirection (* (Math|Vector|Normalize (+ (Math|Vector|Normalize (LocalVariables|GetLLeftDirection)) (Math|Vector|Normalize (LocalVariables|GetLRightDirection)))) (Variables|FieldOfVision|GetExternalRadius)))
        (bind _outhit (Collision|LineTraceByChannel StartPoint (+ StartPoint (LocalVariables|GetLMidDirection)) "TraceTypeQuery1" false 0 "None"))
        ;[1 1 1] SetNewLeftOrRightDirection
        (if (== (.HitActor (Collision|BreakHitResult _outhit)) (LocalVariables|GetLLeftActor))
          (LocalVariables|SetLLeftDirection (LocalVariables|GetLMidDirection))
          (elif (== (.HitActor (Collision|BreakHitResult _outhit)) (LocalVariables|GetLRightVector))
            (LocalVariables|SetLRightDirection (LocalVariables|GetLMidDirection))
            (else
              (Utilities|Array|Insert (LocalVariables|GetLOtherActors) (.HitActor (Collision|BreakHitResult _outhit)))))))))
  (bind _outhit_2 (Collision|LineTraceByChannel (LocalVariables|GetLStartPoint) (+ (LocalVariables|GetLStartPoint) (LocalVariables|GetLLeftDirection)) "TraceTypeQuery1" false 0 (Variables|Debug|GetDrawDebugType) true "(R=0.000000,G=0.084930,B=1.000000,A=1.000000)" "(R=0.000000,G=0.821644,B=1.000000,A=1.000000)" (Variables|Debug|GetDraw%20Time)))
  (Utilities|Array|Add (LocalVariables|GetLNewHits) _outhit_2)
  (bind _outhit_3 (Collision|LineTraceByChannel (LocalVariables|GetLStartPoint) (+ (LocalVariables|GetLStartPoint) (LocalVariables|GetLRightDirection)) "TraceTypeQuery1" false 0 (Variables|Debug|GetDrawDebugType) true "(R=0.000000,G=0.084930,B=1.000000,A=1.000000)" "(R=0.000000,G=0.821644,B=1.000000,A=1.000000)" (Variables|Debug|GetDraw%20Time)))
  (Utilities|Array|Add (LocalVariables|GetLNewHits) _outhit_3)
  (if (!= (Utilities|Array|Length _lotheractors) 0)
    (LocalVariables|SetLLeftActor (Utilities|Array|Get(acopy) _lotheractors))
    (Utilities|Array|RemoveIndex (LocalVariables|GetLOtherActors))
    (LocalVariables|SetLLeftDirection (LocalVariables|GetLRightDirection))
    (LocalVariables|SetLRightDirection _returnvalue)
    (goto _label)
    (else
      (return (LocalVariables|GetLNewHits)))))

(fn Update
  (Variables|Auxiliary|SetStartPoint (+ (Math|Vector|MakeVector 0.0 0.0 (- (Variables|FieldOfVision|GetHeightOfCheck) 1e+02)) (Transformation|GetActorLocation)))
  (Utilities|Array|Clear (Variables|Auxiliary|GetHitResults))
  (Class|ProceduralMeshComponent|ClearAllMeshSections (Variables|Default|GetProceduralMesh)))

(fn CheckActorHigh
  (params (HitResult :type Hit%20Result%20Structure))
  (Variables|Default|SetCurrentHit HitResult)
  ;[1 1 1] Берем нормаль и место столкновения
  (bind _output_get (LocalVariables|SetHitLocation (.Location (Collision|BreakHitResult (Variables|Default|GetCurrentHit)))))
  ;[1 1 1] Поднимаем место трейса на N см и трейсим дальше
  (bind _outhit (Collision|LineTraceByChannel (+ _output_get "0.000000,0.000000,100.000000") (+ (+ _output_get "0.000000,0.000000,100.000000") (* (Math|Vector|GetForwardVector (Math|Rotator|FindLookatRotation (+ _output_get "0.000000,0.000000,100.000000") (Transformation|GetActorLocation))) (* (Variables|FieldOfVision|GetExternalRadius) -1.0))) "TraceTypeQuery1" false 0 "None" true "(R=0.000000,G=0.164826,B=1.000000,A=1.000000)" "(R=0.963607,G=0.000000,B=1.000000,A=1.000000)"))
  (return (and (.bBlockingHit (Collision|BreakHitResult _outhit)) (< (Math|Vector|Distance2D(Vector) (.Location (Collision|BreakHitResult _outhit)) (+ _output_get "0.000000,0.000000,100.000000")) 5.0)) (Math|Vector|MakeVector (.X (Class|KismetMathLibrary|BreakVector3f (.Location (Collision|BreakHitResult _outhit)))) (.Y (Class|KismetMathLibrary|BreakVector3f (.Location (Collision|BreakHitResult _outhit)))) (.Z (Math|Vector|BreakVector (.Location (Collision|BreakHitResult (Variables|Default|GetCurrentHit)))))) (Math|Vector|MakeVector (.X (Class|KismetMathLibrary|BreakVector3f (.TraceEnd (Collision|BreakHitResult _outhit)))) (.Y (Class|KismetMathLibrary|BreakVector3f (.TraceEnd (Collision|BreakHitResult _outhit)))) (.Z (Math|Vector|BreakVector (.Location (Collision|BreakHitResult (Variables|Default|GetCurrentHit)))))) (.bBlockingHit (Collision|BreakHitResult _outhit))))

(fn Initizialize
  (params (HalfAngle :type Float%20%28double-precision%29) (ExternalRadius :type Float%20%28double-precision%29) (InternalRadiusOvVisibility :type Float%20%28double-precision%29))
  (Variables|Default|Setinit true)
  (Variables|FieldOfVision|SetHalfAngle HalfAngle)
  (Variables|FieldOfVision|SetExternalRadius ExternalRadius)
  (Variables|FieldOfVision|SetInternalRadiusOvVisibility InternalRadiusOvVisibility)
  (CallFunction|Start))

(fn SetNewRadius
  (params (ExternalRadius :type Float%20%28double-precision%29) (InternalRadiusOvVisibility :type Float%20%28double-precision%29))
  (Variables|FieldOfVision|SetExternalRadius ExternalRadius)
  (Variables|FieldOfVision|SetInternalRadiusOvVisibility InternalRadiusOvVisibility))