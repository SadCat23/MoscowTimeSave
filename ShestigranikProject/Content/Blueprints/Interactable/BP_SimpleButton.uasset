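; BP_SimpleButton is an interactable button that animates when pressed and can activate a linked actor.
; The activate press event, guarded by a DoOnce node, calls the parent and plays a timeline that slides the button mesh along local Y.
; When the animation finishes, it calls OnPressed and sends ActivateObjectMessage to ActorToActivate if valid.
; A DoOnce flag then either disables the sphere's collision for single use or resets the guard.
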(event EventBeginPlay
  (|CallParentFunction) ; This node is disabled and will not be called.\nDrag off pins to build functionality.
)

(event Collision|EventActorBeginOverlap
  (params (OtherActor :type Actor%20Object%20Reference))
  (|CallParentFunction OtherActor) ; This node is disabled and will not be called.\nDrag off pins to build functionality.
)

(event EventTick
  (params (DeltaSeconds :type Float%20%28single-precision%29))
  (|CallParentFunction DeltaSeconds) ; This node is disabled and will not be called.\nDrag off pins to build functionality.
)

(event EventOnActivateButtonPressed
  (params (Character :type BP%20Base%20Character%20Object%20Reference))
  (bind _actortoactivate (Variables|Default|GetActorToActivate))
  (Utilities|FlowControl|DoOnce false :!label _label
    (:Completed
      (|CallParentFunction Character)
      (bind _offset (Timeline|Timeline PlayFromStart)
        (:Update
          (Transformation|SetRelativeLocation (Variables|Default|GetButtonMesh) (Math|Vector|MakeVector 0.0 _offset 0.0) false false))
        (:Finished
          (Utilities|FlowControl|Sequence
            (:then_0
              (Default|CallOnPressed)
              (Utilities|IsValid _actortoactivate
                (:Is%20Valid
                  (Class|ITriggerableObject|ActivateObject(Message) _actortoactivate))))
            (:then_1
              (if (Variables|Default|GetDoOnce)
                (Collision|SetCollisionEnabled (Variables|Default|GetSphere) "NoCollision")
                (else
                  (goto _label Reset))))))))))

(fn ConstructionScript
  (|CallParentFunction))