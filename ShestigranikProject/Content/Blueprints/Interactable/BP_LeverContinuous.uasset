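; Interactable lever that takes a set activation time to throw and triggers a linked actor on completion.
; Pressing activate plays a timeline, rate-scaled by TimeToActivate, that pitches the Scene component through its swing.
; Interruption reverses the timeline at a faster rate, swinging the lever back.
; The parent's Completed event sends ActivateObjectMessage to a valid ActorToActivate, then disables Sphere collision.
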(event EventBeginPlay
  (|CallParentFunction) ; This node is disabled and will not be called.\nDrag off pins to build functionality.
)

(event Collision|EventActorBeginOverlap
  (params (OtherActor :type Actor%20Object%20Reference))
  (|CallParentFunction OtherActor) ; This node is disabled and will not be called.\nDrag off pins to build functionality.
)

(event EventTick
  (params (DeltaSeconds :type Float%20%28single-precision%29))
  (|CallParentFunction DeltaSeconds) ; This node is disabled and will not be called.\nDrag off pins to build functionality.
)

(event EventCompleted
  (bind _actortoactivate (Variables|Default|GetActorToActivate))
  (|CallParentFunction)
  (Utilities|IsValid _actortoactivate
    (:Is%20Valid
      (Class|ITriggerableObject|ActivateObject(Message) _actortoactivate)
      (Collision|SetCollisionEnabled (Variables|Default|GetSphere) "NoCollision"))))

(event EventInterupted
  (|CallParentFunction)
  (Components|Timeline|SetPlayRate (Variables|Default|GetTimeline) 3.0)
  (bind _newtrack_0 (Timeline|Timeline Reverse)
    (:Update
      (Transformation|SetRelativeRotation (Variables|Default|GetScene) (Math|Rotator|MakeRotator 0.0 (Math|Float|Lerp -4e+01 4e+01 _newtrack_0) 0.0) false false))))

(event EventOnActivateButtonPressed
  (params (Character :type BP%20Base%20Character%20Object%20Reference))
  (|CallParentFunction Character)
  (Components|Timeline|SetPlayRate (Variables|Default|GetTimeline) (/ 1.0 (Variables|Default|GetTimeToActivate)))
  (bind _newtrack_0 (Timeline|Timeline Play)
    (:Update
      (Transformation|SetRelativeRotation (Variables|Default|GetScene) (Math|Rotator|MakeRotator 0.0 (Math|Float|Lerp -4e+01 4e+01 _newtrack_0) 0.0) false false))))

(fn ConstructionScript
  (|CallParentFunction))