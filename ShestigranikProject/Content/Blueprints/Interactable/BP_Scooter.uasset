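; BP_Scooter is an interactable scooter that, once completed, makes a noise and alerts nearby enemies.
; Completion disables its sphere collision, brightens a dynamic material on ElectroS and starts a short one-shot timer.
; When the timer fires, it plays Noise, briefly flashes the emissive power and then sends TriggerEnemyMessage to every actor overlapping TriggerSphere.
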(event Custom|TriggerEnemies
  (Audio|Components|Audio|Play (Variables|Default|GetNoise) 0.0)
  (Rendering|Material|SetScalarParameterValue (Variables|Default|GetMatInst) "EmissivePower" 1e+03 :!class /Script/Engine.MaterialInstanceDynamic)
  (Utilities|FlowControl|Delay 0.1)
  (Rendering|Material|SetScalarParameterValue (Variables|Default|GetMatInst) "EmissivePower" 2e+01 :!class /Script/Engine.MaterialInstanceDynamic)
  (for _array_element (Collision|GetOverlappingActors (Variables|Default|GetTriggerSphere) 0 :!class /Script/Engine.PrimitiveComponent)
    (Class|ITriggerEnemy|TriggerEnemy(Message) _array_element self)))

(event EventBeginPlay
  (|CallParentFunction)
  (bind _returnvalue (Rendering|Material|CreateDynamicMaterialInstance (Variables|Default|GetElectro_S) 0 0 "None" :!class /Script/Engine.PrimitiveComponent))
  (Variables|Default|SetMatInst _returnvalue))

(event Collision|EventActorBeginOverlap
  (params (OtherActor :type Actor%20Object%20Reference))
  (|CallParentFunction OtherActor) ; This node is disabled and will not be called.\nDrag off pins to build functionality.
)

(event EventTick
  (params (DeltaSeconds :type Float%20%28single-precision%29))
  (|CallParentFunction DeltaSeconds) ; This node is disabled and will not be called.\nDrag off pins to build functionality.
)

(event EventCompleted
  (|CallParentFunction)
  (Collision|SetCollisionEnabled (Variables|Default|GetSphere) "NoCollision")
  (Rendering|Material|SetScalarParameterValue (Variables|Default|GetMatInst) "EmissivePower" 5e+01 :!class /Script/Engine.MaterialInstanceDynamic)
  (Utilities|Time|SetTimerbyEvent (delegate Custom|TriggerEnemies) 2.0))

(fn ConstructionScript
  (|CallParentFunction))