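; BP_Task_2_2_2 is an interactable task actor that activates a linked actor when a character presses the activate button.
; The press passes a do-once gate, runs the parent handler, then sends ActivateObjectMessage to ActorToActivate if it is valid.
; The DoOnce flag decides reuse: when set, the Sphere's collision is disabled; otherwise the gate resets for further presses.
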(event EventBeginPlay
  (|CallParentFunction) ; This node is disabled and will not be called.\nDrag off pins to build functionality.
)

(event Collision|EventActorBeginOverlap
  (params (OtherActor :type Actor%20Object%20Reference))
  (|CallParentFunction OtherActor) ; This node is disabled and will not be called.\nDrag off pins to build functionality.
)

(event EventTick
  (params (DeltaSeconds :type Float%20%28single-precision%29))
  (|CallParentFunction DeltaSeconds) ; This node is disabled and will not be called.\nDrag off pins to build functionality.
)

(event EventOnActivateButtonPressed
  (params (Character :type BP%20Base%20Character%20Object%20Reference))
  (bind _actortoactivate (Variables|Default|GetActorToActivate))
  (Utilities|FlowControl|DoOnce false :!label _label
    (:Completed
      (|CallParentFunction Character)
      (Utilities|FlowControl|Sequence
        (:then_0
          (Utilities|IsValid _actortoactivate
            (:Is%20Valid
              (Class|ITriggerableObject|ActivateObject(Message) _actortoactivate))))
        (:then_1
          (if (Variables|Default|GetDoOnce)
            (Collision|SetCollisionEnabled (Variables|Default|GetSphere) "NoCollision")
            (else
              (goto _label Reset))))))))

(fn ConstructionScript
  (|CallParentFunction))