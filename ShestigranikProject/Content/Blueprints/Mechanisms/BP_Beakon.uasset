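; BP_Beakon is a beacon mechanism that rises and lights up when activated, and reverses when deactivated.
; BeginPlay creates a dynamic material instance on the Beacon component.
; One Timeline alpha lifts the Scene component and drives the material's Alpha and emissive strength parameters together.
; ActivateObject plays the Timeline and DeactivateObject reverses it; the direction check on finish leads to no further logic.
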(event EventBeginPlay
  (bind _returnvalue (Rendering|Material|CreateDynamicMaterialInstance (Variables|Default|GetBeacon) 0 0 "None" :!class /Script/Engine.PrimitiveComponent))
  (Variables|Default|SetMatInst _returnvalue))

(event Collision|EventActorBeginOverlap
  (params (OtherActor :type Actor%20Object%20Reference)))

(event EventTick
  (params (DeltaSeconds :type Float%20%28single-precision%29)))

(event EventActivateObject
  (bind _matinst (Variables|Default|GetMatInst))
  (bind (_direction _alpha) (Timeline|Timeline Play)
    (:Update
      (Transformation|SetRelativeLocation (Variables|Default|GetScene) (Math|Vector|Lerp(Vector) "0, 0, 0" "0.000000,0.000000,60.000000" _alpha) false false)
      (Rendering|Material|SetScalarParameterValue _matinst "Alpha" _alpha :!class /Script/Engine.MaterialInstanceDynamic)
      (Rendering|Material|SetScalarParameterValue _matinst "EmissiveStrengh" (* _alpha 5e+01) :!class /Script/Engine.MaterialInstanceDynamic))
    (:Finished
      (switch Utilities|FlowControl|Switch|SwitchonETimelineDirection _direction))))

(event EventDeactivateObject
  (bind _matinst (Variables|Default|GetMatInst))
  (bind (_direction _alpha) (Timeline|Timeline Reverse)
    (:Update
      (Transformation|SetRelativeLocation (Variables|Default|GetScene) (Math|Vector|Lerp(Vector) "0, 0, 0" "0.000000,0.000000,60.000000" _alpha) false false)
      (Rendering|Material|SetScalarParameterValue _matinst "Alpha" _alpha :!class /Script/Engine.MaterialInstanceDynamic)
      (Rendering|Material|SetScalarParameterValue _matinst "EmissiveStrengh" (* _alpha 5e+01) :!class /Script/Engine.MaterialInstanceDynamic))
    (:Finished
      (switch Utilities|FlowControl|Switch|SwitchonETimelineDirection _direction))))

(fn ConstructionScript)