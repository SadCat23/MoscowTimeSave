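; BP_LerpingMechanism is an activatable mechanism actor that moves between its starting position and a TargetLocation component's world position.
; A timeline lerps the actor's location, with play rate set from LerpTime and an optional auto-activate on BeginPlay.
; ActivateObject plays and DeactivateObject reverses it, through two DoOnce gates that reset each other to block repeat calls.
; StopTime and StartTime freeze and resume motion by changing the play rate.
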(event EventBeginPlay
  (Variables|Default|SetDefaultPosition (Transformation|GetActorLocation))
  (Variables|Default|SetTargetPosition (Transformation|GetWorldLocation (Variables|Default|GetTargetLocation)))
  (Components|Timeline|SetPlayRate (Variables|Default|GetLerpTimeline) (/ 1.0 (Variables|Default|GetLerpTime)))
  (if (Variables|Default|GetAutoActivate)
    (CallFunction|ActivateObject)))

(event Collision|EventActorBeginOverlap
  (params (OtherActor :type Actor%20Object%20Reference)))

(event EventTick
  (params (DeltaSeconds :type Float%20%28single-precision%29)))

(event EventActivateObject
  (Utilities|FlowControl|DoOnce false
    (:Completed
      (Utilities|FlowControl|Sequence
        (:then_0
          (bind _newtrack_0 (Timeline|LerpTimeline Play)
            (:Update
              (Transformation|SetActorLocation (Math|Vector|Lerp(Vector) (Variables|Default|GetDefaultPosition) (Variables|Default|GetTargetPosition) _newtrack_0) false false))))
        (:then_1
          (Utilities|FlowControl|DoOnce false) ; enters at Reset
        )))))

(event EventDeactivateObject
  (Utilities|FlowControl|DoOnce false
    (:Completed
      (Utilities|FlowControl|Sequence
        (:then_0
          (bind _newtrack_0 (Timeline|LerpTimeline Reverse)
            (:Update
              (Transformation|SetActorLocation (Math|Vector|Lerp(Vector) (Variables|Default|GetDefaultPosition) (Variables|Default|GetTargetPosition) _newtrack_0) false false))))
        (:then_1
          (Utilities|FlowControl|DoOnce false) ; enters at Reset
        )))))

(event EventStartTime
  (Components|Timeline|SetPlayRate (Variables|Default|GetLerpTimeline) (/ 1.0 (Variables|Default|GetLerpTime))))

(event EventStopTime
  (Components|Timeline|SetPlayRate (Variables|Default|GetLerpTimeline) 0.0))

(fn ConstructionScript)