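; CCTV mechanism that, when activated, makes actors implementing ITriggerEnemy show a vision message while inside its detection radius.
; ActivateObject enables the query-only detection sphere, plays a timeline that fades an indicator material, and starts a cooldown timer that re-arms activation.
; DeactivateObject disables the sphere and reverses the timeline.
; Tick spins the Scene component at a constant rate, independent of activation.
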(event OnComponentBeginOverlap(Sphere)
  (params (OverlappedComponent :type Primitive%20Component%20Object%20Reference) (OtherActor :type Actor%20Object%20Reference) (OtherComp :type Primitive%20Component%20Object%20Reference) (OtherBodyIndex :type Integer) (bFromSweep :type Boolean) (SweepResult :type Hit%20Result%20Structure%20%28by%20ref%29))
  (if (Utilities|DoesObjectImplementInterface OtherActor "/Game/Blueprints/Interfaces/ITriggerEnemy.ITriggerEnemy_C")
    (Class|ITriggerEnemy|ShowVision(Message) OtherActor (Variables|Default|GetShowDuration))))

(event OnComponentEndOverlap(Sphere)
  (params (OverlappedComponent :type Primitive%20Component%20Object%20Reference) (OtherActor :type Actor%20Object%20Reference) (OtherComp :type Primitive%20Component%20Object%20Reference) (OtherBodyIndex :type Integer))
  (if (Utilities|DoesObjectImplementInterface OtherActor "/Game/Blueprints/Interfaces/ITriggerEnemy.ITriggerEnemy_C")
    (Class|ITriggerEnemy|HideVision(Message) OtherActor)))

(event Custom|Reset
  (Utilities|FlowControl|Sequence
    (:then_0
      (Utilities|FlowControl|DoOnce false) ; enters at Reset
    )))

(event EventBeginPlay
  (bind _returnvalue (Rendering|Material|CreateDynamicMaterialInstance (Variables|Default|GetCube2) 0 0 "None" :!class /Script/Engine.PrimitiveComponent))
  (Variables|Default|SetMatInst_Indicator _returnvalue))

(event Collision|EventActorBeginOverlap
  (params (OtherActor :type Actor%20Object%20Reference)))

(event EventTick
  (params (DeltaSeconds :type Float%20%28single-precision%29))
  (Transformation|AddRelativeRotation (Variables|Default|GetScene) (Math|Rotator|MakeRotator 0.0 0.0 (* DeltaSeconds 1e+01)) false false))

(event EventActivateObject
  (Utilities|FlowControl|DoOnce false
    (:Completed
      (Collision|SetCollisionEnabled (Variables|Default|GetSphere) "QueryOnly")
      (bind _returnvalue (Utilities|Time|SetTimerbyEvent (delegate Custom|Reset) (Variables|Default|GetCooldown)))
      (Variables|Default|SetCooldownTimer _returnvalue)
      (bind _alpha (Timeline|Timeline Play)
        (:Update
          (Rendering|Material|SetScalarParameterValue (Variables|Default|GetMatInst_Indicator) "Alpha" _alpha :!class /Script/Engine.MaterialInstanceDynamic))))))

(event EventDeactivateObject
  (Collision|SetCollisionEnabled (Variables|Default|GetSphere) "NoCollision")
  (bind _alpha (Timeline|Timeline Reverse)
    (:Update
      (Rendering|Material|SetScalarParameterValue (Variables|Default|GetMatInst_Indicator) "Alpha" _alpha :!class /Script/Engine.MaterialInstanceDynamic))))

(fn ConstructionScript
  (Collision|SetCollisionEnabled (Variables|Default|GetSphere) "NoCollision")
  (Components|Sphere|SetSphereRadius (Variables|Default|GetSphere) (Variables|Default|GetDetectRadius) true))