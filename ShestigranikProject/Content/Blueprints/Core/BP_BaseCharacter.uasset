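; Base character Blueprint that Init configures from a character data asset: mesh, passive ability and ability set.
; Input triggers first-slot and ultimate abilities, playing montages or reporting failures; ultimates are also added to the game manager's timeline.
; Capsule overlaps track a nearby interactable, which receives interaction press and release messages.
; Events freeze or resume time dilation and cooldowns, and drive ability FX, including a reversible timeline-scaled ring.
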(event OnComponentBeginOverlap(CapsuleComponent)
  (params (OverlappedComponent :type Primitive%20Component%20Object%20Reference) (OtherActor :type Actor%20Object%20Reference) (OtherComp :type Primitive%20Component%20Object%20Reference) (OtherBodyIndex :type Integer) (bFromSweep :type Boolean) (SweepResult :type Hit%20Result%20Structure%20%28by%20ref%29))
  (if (Utilities|DoesObjectImplementInterface OtherActor "/Game/Blueprints/Interfaces/IInteractableObject.IInteractableObject_C")
    (Variables|Default|SetLastInteractableNearby OtherActor)))

(event OnComponentEndOverlap(CapsuleComponent)
  (params (OverlappedComponent :type Primitive%20Component%20Object%20Reference) (OtherActor :type Actor%20Object%20Reference) (OtherComp :type Primitive%20Component%20Object%20Reference) (OtherBodyIndex :type Integer))
  (if (Utilities|DoesObjectImplementInterface OtherActor "/Game/Blueprints/Interfaces/IInteractableObject.IInteractableObject_C")
    (Variables|Default|SetLastInteractableNearby 0)))

(event Custom|StartRemoteControlFX
  (params (Radius :type Float%20%28double-precision%29))
  ;[0.5373 0.5464 1 1 30] AbilityFX
  (bind _returnvalue (Game|AddComponentbyClass "/Script/Engine.StaticMeshComponent" false (Math|Transform|MakeTransform "0.000000,0.000000,-15.000000" "0, 0, 0" "0.000000,0.000000,0.000000")))
  (Components|StaticMesh|SetStaticMesh _returnvalue "/Game/Models/Ring.Ring")
  (Rendering|Material|SetMaterial _returnvalue 0 "/Game/Materials/Effects/MI_RemoteControlZone.MI_RemoteControlZone")
  (bind _output_get (Variables|Default|SetRingMesh _returnvalue))
  (Rendering|SetCastShadow _output_get false)
  (Collision|SetCollisionEnabled _output_get "NoCollision")
  (Variables|ForFX|SetRingRadius Radius)
  (bind (_direction _newtrack_0) (Timeline|Timeline Play)
    (:Update
      (Transformation|SetRelativeScale3D (Variables|Default|GetRingMesh) (Math|Vector|Lerp(Vector) "0, 0, 0" (* "1.000000,1.000000,1.000000" (/ (Variables|ForFX|GetRingRadius) 1e+02)) _newtrack_0)))
    (:Finished
      (switch Utilities|FlowControl|Switch|SwitchonETimelineDirection _direction
        (:Backward
          (Components|DestroyComponent (Variables|Default|GetRingMesh)))))))

(event Custom|StopRemoteControlFX
  ;[0.5373 0.5464 1 1 30] AbilityFX
  (bind (_direction _newtrack_0) (Timeline|Timeline Reverse)
    (:Update
      (Transformation|SetRelativeScale3D (Variables|Default|GetRingMesh) (Math|Vector|Lerp(Vector) "0, 0, 0" (* "1.000000,1.000000,1.000000" (/ (Variables|ForFX|GetRingRadius) 1e+02)) _newtrack_0)))
    (:Finished
      (switch Utilities|FlowControl|Switch|SwitchonETimelineDirection _direction
        (:Backward
          (Components|DestroyComponent (Variables|Default|GetRingMesh)))))))

(event Custom|StartTechSupportFX
  ;[0.5373 0.5464 1 1 30] AbilityFX
  (Audio|PlaySoundatLocation "/Engine/VREditor/Sounds/VR_open_Cue.VR_open_Cue" (Transformation|GetActorLocation) "0, 0, 0" 1.0 1.0 0.0 0 0 0 0)
  (bind _returnvalue (AddComponent|AddNiagaraComponent false))
  (Variables|Default|SetSupportNiagara _returnvalue))

(event Custom|StopTechSupportFX
  ;[0.5373 0.5464 1 1 30] AbilityFX
  (Components|DestroyComponent (Variables|Default|GetSupportNiagara)))

(event Input|EnhancedActionEvents|EnhancedInputActionIA_Interaction
  (params (ActionValue :type Boolean) (ElapsedSeconds :type Float%20%28double-precision%29) (TriggeredSeconds :type Float%20%28double-precision%29) (InputAction :type Input%20Action%20Object%20Reference :default "/Game/Input/Actions/IA_Interaction.IA_Interaction"))
  (bind _lastinteractablenearby (Variables|Default|GetLastInteractableNearby))
  (:Started
    (Utilities|IsValid _lastinteractablenearby
      (:Is%20Valid
        (Class|IInteractableObject|OnActivateButtonPressed(Message) _lastinteractablenearby self)
        (Animation|Montage|PlayMontage (Variables|Character|GetMesh) "/Game/Characters/Mixamo/Animations/Angry_Point_Montage.Angry_Point_Montage"))))
  (:Completed
    (Utilities|IsValid _lastinteractablenearby
      (:Is%20Valid
        (Class|IInteractableObject|OnActivateButtonReleased(Message) _lastinteractablenearby)))))

(event Input|EnhancedActionEvents|EnhancedInputActionIA_FirstSlotAbility
  (params (ActionValue :type Boolean) (ElapsedSeconds :type Float%20%28double-precision%29) (TriggeredSeconds :type Float%20%28double-precision%29) (InputAction :type Input%20Action%20Object%20Reference :default "/Game/Input/Actions/Ability/IA_FirstSlotAbility.IA_FirstSlotAbility"))
  (:Triggered
    (bind (_reasonfailed _returnvalue) (Class|BaseCharacter|TryActivateAbility "FirstAbility"))
    (if _returnvalue
      (Animation|Montage|PlayMontage (Variables|Character|GetMesh) "/Game/Characters/Mixamo/Animations/AbilityActivate_Montage.AbilityActivate_Montage")
      (else
        (Default|CallOnFailedActivateAbility _reasonfailed "FirstAbility" self)))))

(event Input|EnhancedActionEvents|EnhancedInputActionIA_UltimateAbility
  (params (ActionValue :type Boolean) (ElapsedSeconds :type Float%20%28double-precision%29) (TriggeredSeconds :type Float%20%28double-precision%29) (InputAction :type Input%20Action%20Object%20Reference :default "/Game/Input/Actions/Ability/IA_UltimateAbility.IA_UltimateAbility"))
  (bind _da_character (Variables|Default|GetDA_Character))
  (:Triggered
    (bind (_reasonfailed _returnvalue) (Class|BaseCharacter|TryActivateAbility "Ultimate"))
    (if _returnvalue
      (Animation|Montage|PlayMontage (Variables|Character|GetMesh) "/Game/Characters/Mixamo/Animations/Ultimate_Montage.Ultimate_Montage"
        (:then
          (bind _returnvalue_2 (Actor|GetActorOfClass "/Game/Blueprints/Core/GameFramework/BP_GameManager.BP_GameManager_C"))
          (Default|AddUltimateAbilityonTimeline _returnvalue_2 (.Value (Utilities|Map|Find (Variables|/Script/ShestigranikProject.DACharacterData|GetAbilities _da_character) "Ultimate")) _da_character self)))
      (else
        (Default|CallOnFailedActivateAbility _reasonfailed "Ultimate" self)))))

(event EventStartTime
  (Variables|Default|SetCustomTimeDilation 1.0)
  (Class|BaseCharacter|StartCooldowns))

(event EventStopTime
  (Variables|Default|SetCustomTimeDilation 0.0)
  (Class|BaseCharacter|StopCooldowns))

(fn ConstructionScript)

(fn Init
  (params (Data :type DA%20Character%20Data%20Object%20Reference))
  (bind _output_get (Variables|Default|SetDA_Character Data))
  (bind _returnvalue (Game|ConstructObjectfromClass self (Variables|/Script/ShestigranikProject.DAAbilityData|GetAbilityClass (Variables|/Script/ShestigranikProject.DACharacterData|GetPassiveAbility _output_get))))
  (Class|BaseTimeAbility|TryActivate _returnvalue)
  (Components|SkeletalMesh|SetSkeletalMeshAsset (Variables|Character|GetMesh) (Variables|/Script/ShestigranikProject.DACharacterData|GetMesh _output_get))
  (Class|BaseCharacter|SetAbilitiesSet (Variables|/Script/ShestigranikProject.DACharacterData|GetAbilities _output_get)))