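; Level time manager actor that stops and resumes time for a set of actors and runs an episode countdown tied to a character index.
; ActivateObject and DeactivateObject play timelines that drive each actor's CustomTimeDilation, or send start/stop messages to ITimeRelativeActor implementers.
; The looping one-second timer starts paused and toggles when those timelines finish.
; UpdateTime decrements the seconds, updates the timer widget and broadcasts updates or timer end.
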(event Custom|UpdateTime
  (bind _result (Math|Float|DecrementFloat (Variables|Default|GetSecondsRemaining))
    (:%20%20
      (Development|PrintString (Utilities|String|ToString(Float) _result))
      (if (<= _result 0.0)
        (Default|CallTimerEnd)
        (Utilities|Time|ClearandInvalidateTimerbyHandle (Variables|Default|GetTimer))
        (else
          (CallFunction|UpdateWidget)
          (Default|CallOnTimeUpdate (Variables|Default|GetSecondsRemaining) (Variables|Default|GetCharIndex)))))))

(event Custom|UpdateWidget
  (bind _timerwidget (Variables|Default|GetTimerWidget))
  (bind _secondsremaining (Variables|Default|GetSecondsRemaining))
  (Utilities|IsValid _timerwidget
    (:Is%20Valid
      (Default|SetTime _timerwidget _secondsremaining (Variables|Default|GetTimerColor))
      (Default|SetProgress _timerwidget (Variables|Default|GetCharIndex) (- 1.0 (/ _secondsremaining (Variables|Default|GetSecondsForEpisode)))))))

(event EventBeginPlay
  (bind _returnvalue (Utilities|Time|SetTimerbyEvent (EventDispatchers|CreateEvent :!event Custom|UpdateTime) 1.0 true))
  (bind _output_get (Variables|Default|SetTimer _returnvalue))
  (Utilities|Time|PauseTimerbyHandle _output_get))

(event Collision|EventActorBeginOverlap
  (params (OtherActor :type Actor%20Object%20Reference)))

(event EventTick
  (params (DeltaSeconds :type Float%20%28single-precision%29)))

(event EventActivateObject
  (bind _timetimeline (Timeline|Timeline Play)
    (:Update
      (for _array_element (Variables|Default|GetActors)
        (if (Utilities|DoesObjectImplementInterface _array_element "/Game/Blueprints/Interfaces/ITimeRelativeActor.ITimeRelativeActor_C")
          (Class|ITimeRelativeActor|StartTime(Message) _array_element)
          (else
            (Utilities|IsValid _array_element
              (:Is%20Valid
                (Variables|/Script/Engine.Actor|SetCustomTimeDilation _array_element _timetimeline)))))))
    (:Finished
      (Utilities|Time|UnpauseTimerbyHandle (Variables|Default|GetTimer))
      (Default|CallTimeReturned))))

(event EventDeactivateObject
  (bind _timetimeline (Timeline|Timeline_0 Play)
    (:Update
      (for _array_element (Variables|Default|GetActors)
        (if (Utilities|DoesObjectImplementInterface _array_element "/Game/Blueprints/Interfaces/ITimeRelativeActor.ITimeRelativeActor_C")
          (Class|ITimeRelativeActor|StopTime(Message) _array_element)
          (else
            (Utilities|IsValid _array_element
              (:Is%20Valid
                (Variables|/Script/Engine.Actor|SetCustomTimeDilation _array_element _timetimeline)))))))
    (:Finished
      (Utilities|Time|PauseTimerbyHandle (Variables|Default|GetTimer))
      (Default|CallTimeStopped))))

(fn ConstructionScript
  (Variables|Default|SetSecondsRemaining (Variables|Default|GetSecondsForEpisode)))

(fn SetCharIndex
  (params (CharIndex :type Integer))
  (Variables|Default|SetCharIndex CharIndex))