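; BP_MoscowGI, by its name the game instance, holds the current level phase and persists whether the tutorial is finished.
; Get and set functions expose the phase index, which is kept only in a variable.
; The tutorial flag goes through a BP_SaveTutorial save object in the "TutorialSave" slot.
; Each write creates a fresh save object, and reads return false when the load or cast fails.
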(fn SetCurrentLevelPhase
  (params (Index :type Integer))
  (Variables|Default|SetCurrentPhase Index))

(fn GetCurrentLevelPhase
  (return (Variables|Default|GetCurrentPhase)))

(fn GetTutorialFinish
  (bind _returnvalue (SaveGame|LoadGamefromSlot "TutorialSave"))
  (bind _asbp_save_tutorial (Utilities|Casting|CastToBP_SaveTutorial _returnvalue)
    (:then
      (return (Variables|/Game/Blueprints/Core/BP_SaveTutorial.BP_SaveTutorial_C|GetFinishTutorial _asbp_save_tutorial)))
    (:CastFailed
      (return false))))

(fn SetTutorialFinish
  (params (FinishTutorial :type Boolean))
  (bind _returnvalue (SaveGame|CreateSaveGameObject "/Game/Blueprints/Core/BP_SaveTutorial.BP_SaveTutorial_C"))
  (Variables|/Game/Blueprints/Core/BP_SaveTutorial.BP_SaveTutorial_C|SetFinishTutorial _returnvalue FinishTutorial)
  (SaveGame|SaveGametoSlot _returnvalue "TutorialSave"))