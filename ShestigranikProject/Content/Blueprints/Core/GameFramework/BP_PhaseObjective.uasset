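; Phase objective trigger that stays hidden and non-colliding until its required number of tasks is done.
; Each ActivateObject call decrements the remaining task count, and at zero enables the Box query collision and shows the contour mesh.
; A BP_BaseCharacter overlapping the Box marks the objective complete, calls OnCompleted with PlayerIndex and plays a sound.
; ReturnIsComplete exposes the completion state, while SecondActivate is left empty.
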(event OnComponentBeginOverlap(Box)
  (params (OverlappedComponent :type Primitive%20Component%20Object%20Reference) (OtherActor :type Actor%20Object%20Reference) (OtherComp :type Primitive%20Component%20Object%20Reference) (OtherBodyIndex :type Integer) (bFromSweep :type Boolean) (SweepResult :type Hit%20Result%20Structure%20%28by%20ref%29))
  (Utilities|Casting|CastToBP_BaseCharacter OtherActor)
  (Variables|Default|SetIsComplete true)
  (Default|CallOnCompleted (Variables|Default|GetPlayerIndex))
  (Rendering|SetVisibility (Variables|Default|GetRoundedCubeContur) true false)
  (Audio|PlaySoundatLocation "/Engine/VREditor/Sounds/UI/Dockable_Window_Close.Dockable_Window_Close" (Transformation|GetActorLocation) "0, 0, 0" 0.7 1.0 0.0 0 0 0 0))

(event EventBeginPlay
  (Variables|Default|SetTasksRemaining (Variables|Default|GetTasksCount))
  (Rendering|SetVisibility (Variables|Default|GetRoundedCubeContur) false false)
  (Collision|SetCollisionEnabled (Variables|Default|GetBox) "NoCollision"))

(event Collision|EventActorBeginOverlap
  (params (OtherActor :type Actor%20Object%20Reference)))

(event EventTick
  (params (DeltaSeconds :type Float%20%28single-precision%29)))

(event EventActivateObject
  (bind _result (Math|Integer|DecrementInt (Variables|Default|GetTasksRemaining))
    (:%20%20
      (if (<= _result 0)
        (Collision|SetCollisionEnabled (Variables|Default|GetBox) "QueryOnly")
        (Rendering|SetVisibility (Variables|Default|GetRoundedCubeContur) true false)))))

(event EventSecondActivate)

(fn ConstructionScript)

(fn ReturnIsComplete
  (return (Variables|Default|GetIsComplete)))