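; BP_Noise is an ability that temporarily halves the view radius of enemies on the current timeline.
; On execute it gathers BP_BaseEnemy actors from the current time manager, obtained through BP_GameManager, and shrinks each one's radius.
; A five-second timer then restores each radius from the enemy's default config and finishes the ability.
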(event Custom|Finish
  (for _array_element (Variables|Default|GetOut%20Actors)
    (Default|UpdateViewRadius _array_element (.MaxViewRadius (Utilities|Struct|BreakST_Enemy (Variables|/Game/AI/BP_BaseEnemy.BP_BaseEnemy_C|GetDefaultEnemyConfig _array_element)))))
  (Class|BaseTimeAbility|FinishAbility))

(event EventOnActivate
  (Class|BaseTimeAbility|TryExecute))

(event EventOnExecute
  (Utilities|Time|SetTimerbyEvent (delegate Custom|Finish) 5.0)
  (bind _outactors (CallFunction|GetAllEnemyonCurentTimeLine))
  (bind _output_get (Variables|Default|SetOut%20Actors _outactors))
  (for _array_element _output_get
    (Default|UpdateViewRadius _array_element (* (Variables|/Game/AI/BP_BaseEnemy.BP_BaseEnemy_C|GetMaxViewRadius _array_element) 0.5))))

(fn GetAllEnemyonCurentTimeLine
  (bind _returnvalue (Actor|GetActorOfClass "/Game/Blueprints/Core/GameFramework/BP_GameManager.BP_GameManager_C"))
  (bind _timemanager (Default|ReturnCurrentTimeManager _returnvalue))
  (for _array_element (Variables|/Game/Blueprints/Core/GameFramework/BP_LevelTimeManager.BP_LevelTimeManager_C|GetActors _timemanager)
    (bind _asbp_base_enemy (Utilities|Casting|CastToBP_BaseEnemy _array_element))
    (Utilities|Array|Add (LocalVariables|GetOut) _asbp_base_enemy))
  (return (LocalVariables|GetOut)))