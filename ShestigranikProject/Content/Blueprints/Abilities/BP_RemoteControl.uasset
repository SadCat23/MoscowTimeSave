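; Remote control ability that lets the owning character trigger the nearest BaseInteractable within a radius for a limited time.
; A looping timer sphere-traces vertically around the owner, collecting interactables whose sphere component is hit.
; Set differences untrigger objects leaving range; the closest by 2D distance is remote-triggered and stored on the character, and the others are untriggered.
; A Niagara beam follows the target, and finishing clears timer, effects and targets.
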(event Custom|Scan
  (bind _returnvalue (Class|BaseTimeAbility|GetOwnerLocation))
  (bind _returnvalue_2 (Class|BaseTimeAbility|GetOwnerCharacter))
  (bind _beam (Variables|Default|GetBeam))
  (bind _returnvalue_3 (Transformation|GetActorUpVector _returnvalue_2))
  (bind _returnvalue_4 (* _returnvalue_3 500))
  (Variables|Default|SetLastInteractObjects (Variables|Default|GetInteractObjects))
  (Utilities|Set|Clear (Variables|Default|GetInteractObjects))
  (bind _outhits (Collision|MultiSphereTraceForObjects (+ _returnvalue_4 _returnvalue) (- _returnvalue _returnvalue_4) (Variables|Default|GetRadius) (Utilities|Array|MakeArray "ObjectTypeQuery2") false 0 "None" true "(R=0.000000,G=1.000000,B=0.973481,A=1.000000)" "(R=1.000000,G=0.003930,B=0.000000,A=1.000000)" 0.1))
  (for _array_element _outhits
    (bind _asbase_interactable (Utilities|Casting|CastToBaseInteractable (.HitActor (Collision|BreakHitResult _array_element))))
    (if (== (.HitComponent (Collision|BreakHitResult _array_element)) (Variables|/Game/Blueprints/Interactable/Base/BaseInteractable.BaseInteractable_C|GetSphere _asbase_interactable))
      (Utilities|Set|Add (Variables|Default|GetInteractObjects) _asbase_interactable)))
  (CallFunction|ClearOldTrigger)
  (bind _output (CallFunction|GetNearbyObject))
  (bind _output_get (Variables|Default|SetLastInteractableObj _output))
  (Utilities|IsValid _output
    (:Is%20Valid
      (Niagara|SetNiagaraVariable(Vector3) _beam "User.BeamEnd" (Transformation|GetActorLocation _output_get))
      (Default|RemoteTriger _output)
      (Variables|/Game/Blueprints/Core/BP_BaseCharacter.BP_BaseCharacter_C|SetLastInteractableNearby (.AsBP%20Base%20Character (Utilities|Casting|CastToBP_BaseCharacter (Class|BaseTimeAbility|GetOwnerCharacter))) _output)
      (CallFunction|UnTrigerFarObject _output (Variables|Default|GetInteractObjects)))
    (:Is%20Not%20Valid
      (Niagara|SetNiagaraVariable(Vector3) _beam "User.BeamEnd" (Transformation|GetActorLocation (Class|BaseTimeAbility|GetOwnerCharacter))))))

(event Custom|OnFinish
  (bind _returnvalue (Class|BaseTimeAbility|GetOwnerCharacter))
  (bind _asbp_base_character (Utilities|Casting|CastToBP_BaseCharacter _returnvalue))
  (Utilities|Time|ClearandInvalidateTimerbyHandle (Variables|Default|GetScanTimer))
  (Utilities|Set|Clear (Variables|Default|GetInteractObjects))
  (CallFunction|ClearOldTrigger)
  (Components|DestroyComponent (Variables|Default|GetBeam))
  (Default|StopRemoteControlFX _asbp_base_character)
  (if (== (Variables|/Game/Blueprints/Core/BP_BaseCharacter.BP_BaseCharacter_C|GetLastInteractableNearby _asbp_base_character) (Variables|Default|GetLastInteractableObj))
    (Variables|/Game/Blueprints/Core/BP_BaseCharacter.BP_BaseCharacter_C|SetLastInteractableNearby _asbp_base_character 0))
  (Class|BaseTimeAbility|FinishAbility))

(event EventOnActivate
  (Class|BaseTimeAbility|TryExecute))

(event EventOnExecute
  (bind _returnvalue (Utilities|Time|SetTimerbyEvent (EventDispatchers|CreateEvent :!event Custom|Scan) 0.1 true))
  (Variables|Default|SetScanTimer _returnvalue)
  (Utilities|Time|SetTimerbyEvent (EventDispatchers|CreateEvent :!event Custom|OnFinish) 1e+01)
  (bind _asbp_base_character (Utilities|Casting|CastToBP_BaseCharacter (Class|BaseTimeAbility|GetOwnerCharacter)))
  (Utilities|FlowControl|Sequence
    (:then_0
      (bind _returnvalue_2 (Niagara|SpawnSystemAttached "/Game/Blueprints/Niagara/NS_ControlBeam.NS_ControlBeam" (Variables|/Script/Engine.Character|GetMesh _asbp_base_character) "None" "0, 0, 0" "0, 0, 0" "KeepRelativeOffset" false))
      (bind _output_get (Variables|Default|SetBeam _returnvalue_2))
      (Niagara|SetNiagaraVariable(Vector3) _output_get "User.BeamEnd" (Transformation|GetActorLocation (Class|BaseTimeAbility|GetOwnerCharacter))))
    (:then_1
      (Default|StartRemoteControlFX _asbp_base_character (Variables|Default|GetRadius)))))

(fn ClearOldTrigger
  (bind _result (Utilities|Set|Difference (Variables|Default|GetLastInteractObjects) (Variables|Default|GetInteractObjects)))
  (bind _result_2 (Utilities|Set|ToArray _result))
  (for _array_element _result_2
    (Default|UnTrigger _array_element)))

(fn GetNearbyObject
  (bind _interactobjects (Variables|Default|GetInteractObjects))
  (if (Utilities|Set|IsEmpty _interactobjects)
    (return 0)
    (else
      (bind _result (Utilities|Set|ToArray _interactobjects))
      (bind _output_get (LocalVariables|SetArrayObject _result))
      (for _array_element _output_get
        (Utilities|Array|Add (LocalVariables|GetDistances) (Math|Vector|Distance2D(Vector) (Class|BaseTimeAbility|GetOwnerLocation) (Transformation|GetActorLocation _array_element))))
      (return (Utilities|Array|Get(acopy) (LocalVariables|GetArrayObject) (.IndexOfMinValue (Math|Float|MinOfFloatArray (LocalVariables|GetDistances))))))))

(fn UnTrigerFarObject
  (params (InputPin :type Base%20Interactable%20Object%20Reference) (ScanArray :type Set%20of%20Base%20Interactable%20Object%20References))
  (bind _output_get (LocalVariables|SetNewLocalVar ScanArray))
  (Utilities|Set|Remove _output_get InputPin)
  (bind _result (Utilities|Set|ToArray (LocalVariables|GetNewLocalVar)))
  (for _array_element _result
    (Default|UnTrigger _array_element)))