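; BP_TechSupport is an ability that temporarily halves the owning character's alarm coefficient (CoefAlarm).
; Activation calls TryExecute; execution starts a ten-second one-shot timer, lowers the coefficient on BP_BaseCharacter and starts the tech support FX.
; Finish resets the coefficient to its hardcoded default of one rather than a saved value, stops the FX and ends the ability.
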(event Custom|Finish
  (bind _asbp_base_character (Utilities|Casting|CastToBP_BaseCharacter (Class|BaseTimeAbility|GetOwnerCharacter)))
  (Variables|/Game/Blueprints/Core/BP_BaseCharacter.BP_BaseCharacter_C|SetCoefAlarm _asbp_base_character 1.0)
  (Default|StopTechSupportFX _asbp_base_character)
  (Class|BaseTimeAbility|FinishAbility))

(event EventOnActivate
  (Class|BaseTimeAbility|TryExecute))

(event EventOnExecute
  (Utilities|Time|SetTimerbyEvent (EventDispatchers|CreateEvent :!event Custom|Finish) 1e+01)
  (bind _asbp_base_character (Utilities|Casting|CastToBP_BaseCharacter (Class|BaseTimeAbility|GetOwnerCharacter)))
  (Variables|/Game/Blueprints/Core/BP_BaseCharacter.BP_BaseCharacter_C|SetCoefAlarm _asbp_base_character 0.5)
  (Default|StartTechSupportFX _asbp_base_character))