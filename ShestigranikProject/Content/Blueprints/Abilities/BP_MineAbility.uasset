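; Mine-placing ability that drops a BP_Mine on the surface beneath the owning character.
; Activation immediately calls TryExecute, and OnExecute runs a Visibility line trace along the character's up axis, from above to below its location, ignoring the character.
; On a hit it spawns the mine at the impact location and finishes the ability; a miss does neither.
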(event EventOnExecute
  (bind _returnvalue (Class|BaseTimeAbility|GetOwnerLocation))
  (bind _returnvalue_2 (Class|BaseTimeAbility|GetOwnerCharacter))
  (bind _returnvalue_3 (Transformation|GetActorUpVector _returnvalue_2))
  (bind _returnvalue_4 (* _returnvalue_3 500))
  (bind (_outhit _returnvalue_5) (Collision|LineTraceByChannel (+ _returnvalue_4 _returnvalue) (- _returnvalue _returnvalue_4) "TraceTypeQuery1" false (Utilities|Array|MakeArray (Class|BaseTimeAbility|GetOwnerCharacter)) "None"))
  (if _returnvalue_5
    (Game|SpawnActorfromClass "/Game/Blueprints/Abilities/Actors/BP_Mine.BP_Mine_C" (Math|Transform|MakeTransform (.Location (Collision|BreakHitResult _outhit)) "0, 0, 0" "1.000000,1.000000,1.000000") "Undefined" 0 0)
    (Class|BaseTimeAbility|FinishAbility)))

(event EventOnActivate
  (Class|BaseTimeAbility|TryExecute))