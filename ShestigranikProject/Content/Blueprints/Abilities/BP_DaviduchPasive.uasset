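; Passive ability for the Daviduch character that scales the owning character's movement speeds.
; Activation tries to execute right away, and execution casts the owner to BP_BaseCharacter.
; It multiplies the current walking, crouching and running speeds by Coef through UpdateMovementSpeeds, then finishes the ability.
; The change is a one-shot multiplication with no revert in this graph.
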(event EventOnActivate
  (Class|BaseTimeAbility|TryExecute))

(event EventOnExecute
  (bind _coef (Variables|Default|GetCoef))
  (bind _asbp_base_character (Utilities|Casting|CastToBP_BaseCharacter (Class|BaseTimeAbility|GetOwnerCharacter)))
  (Class|BaseCharacter|UpdateMovementSpeeds _asbp_base_character (* _coef (Variables|/Script/ShestigranikProject.BaseCharacter|GetWalkingSpeed _asbp_base_character)) (* (Variables|/Script/ShestigranikProject.BaseCharacter|GetCrouchingSpeed _asbp_base_character) _coef) (* (Variables|/Script/ShestigranikProject.BaseCharacter|GetRunningSpeed _asbp_base_character) _coef))
  (Class|BaseTimeAbility|FinishAbility))