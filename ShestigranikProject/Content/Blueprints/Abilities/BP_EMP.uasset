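; EMP ability that temporarily disables all enemies on the current timeline.
; On execute it gathers BP_BaseEnemy actors from the time manager returned by BP_GameManager, then puts each to sleep, blinds it, plays EMP effects and zeroes its alarm value.
; A five-second timer then stops sleep and effects, clears blindness on the cached enemies and finishes the ability, without restoring alarm values.
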(event Custom|Finish
  (for _array_element (Variables|Default|GetOut%20Actors)
    (Default|StopEMPFX _array_element)
    (Default|StopSleep _array_element)
    (Variables|/Game/AI/BP_BaseEnemy.BP_BaseEnemy_C|SetBlind _array_element false))
  (Class|BaseTimeAbility|FinishAbility))

(event EventOnActivate
  (Class|BaseTimeAbility|TryExecute))

(event EventOnExecute
  (Utilities|Time|SetTimerbyEvent (delegate Custom|Finish) 5.0)
  (bind _outactors (CallFunction|GetAllEnemyonCurentTimeLine))
  (bind _output_get (Variables|Default|SetOut%20Actors _outactors))
  (for _array_element _output_get
    (Default|StartEMPFX _array_element)
    (Default|StartSleep _array_element)
    (Variables|/Game/AI/BP_BaseEnemy.BP_BaseEnemy_C|SetBlind _array_element true)
    (Default|SetNewAlarmValue _array_element 0.0)))

(fn GetAllEnemyonCurentTimeLine
  (bind _returnvalue (Actor|GetActorOfClass "/Game/Blueprints/Core/GameFramework/BP_GameManager.BP_GameManager_C"))
  (bind _timemanager (Default|ReturnCurrentTimeManager _returnvalue))
  (for _array_element (Variables|/Game/Blueprints/Core/GameFramework/BP_LevelTimeManager.BP_LevelTimeManager_C|GetActors _timemanager)
    (bind _asbp_base_enemy (Utilities|Casting|CastToBP_BaseEnemy _array_element))
    (Utilities|Array|Add (LocalVariables|GetOut) _asbp_base_enemy))
  (return (LocalVariables|GetOut)))