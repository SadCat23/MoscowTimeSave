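; BP_Distract is a character ability that distracts nearby enemies.
; On activation it sphere-traces pawns along the owner's vertical axis with debug drawing, collects BP_BaseEnemy hits into a set, starts their distract FX and calls TryExecute.
; On execution it resets each collected enemy's alarm to zero, blinds them and finishes the ability.
; The Enemy set is not cleared in this graph.
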(event EventOnActivate
  (bind _returnvalue (Class|BaseTimeAbility|GetOwnerLocation))
  (bind _returnvalue_2 (Class|BaseTimeAbility|GetOwnerCharacter))
  (bind _returnvalue_3 (Transformation|GetActorUpVector _returnvalue_2))
  (bind _returnvalue_4 (* _returnvalue_3 500))
  (bind _outhits (Collision|MultiSphereTraceForObjects (+ _returnvalue_4 _returnvalue) (- _returnvalue _returnvalue_4) 4e+02 (Utilities|Array|MakeArray "ObjectTypeQuery3") false 0 "ForDuration" true "(R=0.000000,G=1.000000,B=0.973481,A=1.000000)" "(R=1.000000,G=0.003930,B=0.000000,A=1.000000)" 2.0))
  (for _array_element _outhits
    (bind _asbp_base_enemy (Utilities|Casting|CastToBP_BaseEnemy (.HitActor (Collision|BreakHitResult _array_element))))
    (Utilities|Set|Add (Variables|Default|GetEnemy) _asbp_base_enemy)
    (Default|StartDistractFX _asbp_base_enemy))
  (Class|BaseTimeAbility|TryExecute))

(event EventOnExecute
  (bind _result (Utilities|Set|ToArray (Variables|Default|GetEnemy)))
  (for _array_element _result
    (Default|SetNewAlarmValue _array_element 0.0)
    (Default|SetBlinded _array_element 1.0))
  (Class|BaseTimeAbility|FinishAbility))