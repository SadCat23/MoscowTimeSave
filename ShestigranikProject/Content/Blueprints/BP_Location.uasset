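; BP_Location is a location marker actor shown as a billboard sprite, with active and hover states.
; SetActive swaps the sprite between the Location and Vector images, and BeginPlay applies the initial Active value.
; StartHover plays a timeline that scales the actor from its cached starting scale up to one and a half times, and EndHover reverses it.
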(event Custom|StartHover
  (bind _newtrack_0 (Timeline|Timeline Play)
    (:Update
      (Transformation|SetActorScale3D (Math|Vector|Lerp(Vector) (Variables|Default|GetBeginScale) (* (Variables|Default|GetBeginScale) 1.5) _newtrack_0)))))

(event Custom|EndHover
  (bind _newtrack_0 (Timeline|Timeline Reverse)
    (:Update
      (Transformation|SetActorScale3D (Math|Vector|Lerp(Vector) (Variables|Default|GetBeginScale) (* (Variables|Default|GetBeginScale) 1.5) _newtrack_0)))))

(event Custom|SetActive
  (params (IsActive :type Boolean))
  (Rendering|Components|Sprite|SetSprite (Variables|Default|GetBillboard) (select IsActive "/Game/Textures/UI/Resource/location.location" "/Game/Textures/UI/Resource/Vector.Vector")))

(event EventBeginPlay
  (Variables|Default|SetBeginScale (Transformation|GetActorScale3D))
  (CallFunction|SetActive (Variables|Default|GetActive)))

(event Collision|EventActorBeginOverlap
  (params (OtherActor :type Actor%20Object%20Reference)))

(event EventTick
  (params (DeltaSeconds :type Float%20%28single-precision%29)))

(fn ConstructionScript)